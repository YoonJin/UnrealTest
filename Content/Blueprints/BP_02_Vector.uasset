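; BP_02_Vector is an actor Blueprint that demonstrates moving an actor with vector math.
; On BeginPlay it makes a single, unswept location change, a short step along the normalized forward vector of its own rotation.
; Two unconnected variants remain in the event graph: an offset along world X and a step along the forward vector of a fixed yaw rotation.
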(event `self.ReceiveBeginPlay`
  (`self.K2_SetActorLocation` (+ (`self.K2_GetActorLocation`) (* (`KismetMathLibrary.Normal` (`KismetMathLibrary.GetForwardVector` (`self.K2_GetActorRotation`))) 10.0))))

(fn `UserConstructionScript`)