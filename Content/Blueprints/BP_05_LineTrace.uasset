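; BP_05_LineTrace is a demo actor that traces a line between two BP_05_DrawLine actors and recolors the player when it crosses that line.
; BeginPlay gathers those actors and puts a dynamic material instance on the player character's mesh.
; Each Tick runs a debug-drawn object trace for Pawns, and a BP_Player_2 hit sets BodyColor to a new random color.
; The DrawLine helper and an actor-name printing loop are left unconnected.
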(event `self.ReceiveBeginPlay`
  (bind _outactors (`GameplayStatics.GetAllActorsOfClass` "/Game/Blueprints/BP_05_DrawLine.BP_05_DrawLine_C"))
  (set `self.Lines` _outactors)
  (bind _returnvalue (`KismetMaterialLibrary.CreateDynamicMaterialInstance` (`PrimitiveComponent.GetMaterial` (`Character.Mesh` (`GameplayStatics.GetPlayerCharacter` 0)) 0)))
  (set `self.BodyMaterial` _returnvalue)
  (`PrimitiveComponent.SetMaterial` (`Character.Mesh` (`GameplayStatics.GetPlayerCharacter` 0)) 0 (`self.BodyMaterial`)))

(event `self.ReceiveTick`
  (params (DeltaSeconds :type "Float (single-precision)"))
  (bind (_outhit _returnvalue) (`KismetSystemLibrary.LineTraceSingleForObjects` (`self.K2_GetActorLocation` (`|GetArrayItem` (`self.Lines`))) (`self.K2_GetActorLocation` (`|GetArrayItem` (`self.Lines`) 1)) (`|MakeArray` "ObjectTypeQuery3" :!type "EObjectTypeQuery Enum") false (`self.Lines`) "ForOneFrame" true (struct :`G` 1.0 :`A` 1.0) (struct :`R` 1.0 :`A` 1.0)))
  (if _returnvalue
    (bind _asbp_player_2 (cast `/Game/Player/BP_Player_2` (`.HitActor` (`GameplayStatics.BreakHitResult` _outhit))))
    (`/Engine/EditorBlueprintResources/StandardMacros.IsValid` _asbp_player_2
      (:`Is Valid`
        (`MaterialInstanceDynamic.SetVectorParameterValue` (`self.BodyMaterial`) "BodyColor" (make `LinearColor` (`KismetMathLibrary.RandomFloatInRange` 0.0 1.0) (`KismetMathLibrary.RandomFloatInRange` 0.0 1.0) (`KismetMathLibrary.RandomFloatInRange` 0.0 1.0)))))))

(fn `DrawLine`
  (params (Duration :type "Float (double-precision)"))
  (`KismetSystemLibrary.DrawDebugLine` (`self.K2_GetActorLocation` (`|GetArrayItem` (`self.Lines`))) (`self.K2_GetActorLocation` (`|GetArrayItem` (`self.Lines`) 1)) (struct :`G` 0.050516 :`B` 1.0 :`A` 1.0) Duration))

(fn `UserConstructionScript`)