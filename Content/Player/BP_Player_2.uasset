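; Third-person player character with camera-relative movement, look, jump, spring-arm zoom, a walk-speed toggle and a drawable sword.
; BeginPlay spawns BP_Sword into a holster socket; drawing or sheathing locks movement and switches between controller-yaw and movement-oriented rotation.
; Separate grab, ungrab and completion events, with no callers here, move the sword between sockets and update state.
; Attacks play a melee montage only while drawn, gated by a flag that EndAttack clears.
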(event `self.ReceiveBeginPlay`
  (bind _returnvalue (`|SpawnActorFromClass` "/Game/Weapons/BP_Sword.BP_Sword_C" (`KismetMathLibrary.MakeTransform` (0.0 0.0 0.0)) "Undefined" "OverrideRootScale" self null))
  (bind _output_get (set `self.Sword` _returnvalue))
  (`self.K2_AttachToComponent` _output_get (`self.Mesh`) "Holster_Sword" "KeepRelative" "KeepRelative" "KeepRelative" true))

(event `InputAxis|MoveForward`
  (params (AxisValue :type "Float (single-precision)"))
  (bind (_returnvalue_roll _returnvalue_pitch _returnvalue_yaw) (`KismetMathLibrary.BreakRotator` (`self.GetControlRotation`)))
  (if (`self.canMove`)
    (`self.AddMovementInput` (`KismetMathLibrary.Vector_Normal2D` (`KismetMathLibrary.GetForwardVector` (`KismetMathLibrary.MakeRotator` 0.0 0.0 _returnvalue_yaw))) AxisValue)))

(event `InputAxis|MoveRight`
  (params (AxisValue :type "Float (single-precision)"))
  (bind (_returnvalue_roll _returnvalue_pitch _returnvalue_yaw) (`KismetMathLibrary.BreakRotator` (`self.GetControlRotation`)))
  (if (`self.canMove`)
    (`self.AddMovementInput` (`KismetMathLibrary.Vector_Normal2D` (`KismetMathLibrary.GetRightVector` (`KismetMathLibrary.MakeRotator` 0.0 0.0 _returnvalue_yaw))) AxisValue)))

(event `InputAction|Walking`
  (params (Key :type "Key Structure"))
  (bind _charactermovement (`self.CharacterMovement`))
  (:`Pressed`
    (set `CharacterMovementComponent.MaxWalkSpeed` 400.0 _charactermovement))
  (:`Released`
    (set `CharacterMovementComponent.MaxWalkSpeed` 600.0 _charactermovement)))

(event `InputAxis|Turn`
  (params (AxisValue :type "Float (single-precision)"))
  (`self.AddControllerYawInput` AxisValue))

(event `InputAxis|Lookup`
  (params (AxisValue :type "Float (single-precision)"))
  (`self.AddControllerPitchInput` AxisValue))

(event `Key|SpaceBar`
  (params (Key :type "Key Structure"))
  (:`Pressed`
    (if (`self.canMove`)
      (`self.Jump`)))
  (:`Released`
    (`self.StopJumping`)))

(event `InputAxis|Zoom`
  (params (AxisValue :type "Float (single-precision)"))
  (set `SpringArmComponent.TargetArmLength` (`KismetMathLibrary.FClamp` (+ (* AxisValue (`self.ZoomSpeed`)) (`SpringArmComponent.TargetArmLength` (`self.SpringArm`))) 100.0 600.0) (`self.SpringArm`)))

(event `InputAction|Sword`
  (params (Key :type "Key Structure"))
  (:`Pressed`
    (if (`self.Drawn`)
      (`self.Sheath Sword`)
      (else
        (`self.Equip Sword`)))))

(event `Equip Sword`
  (set `self.Drawing` true)
  (set `self.canMove` false)
  (set `self.bUseControllerRotationYaw` true)
  (set `CharacterMovementComponent.bOrientRotationToMovement` false (`self.CharacterMovement`)))

(event `Equipped Sword`
  (set `self.Drawing` false)
  (set `self.canMove` true)
  (set `self.Drawn` true))

(event `Sheath Sword`
  (set `self.Sheathing` true)
  (set `self.canMove` false)
  (set `self.bUseControllerRotationYaw` false)
  (set `CharacterMovementComponent.bOrientRotationToMovement` true (`self.CharacterMovement`)))

(event `Sheathed Sword`
  (set `self.Sheathing` false)
  (set `self.canMove` true)
  (set `self.Drawn` false))

(event `GrabSword`
  (`self.K2_AttachToComponent` (`self.Sword`) (`self.Mesh`) "Sword" "KeepRelative" "KeepRelative" "KeepRelative" true))

(event `Ungrab Sword`
  (`self.K2_AttachToComponent` (`self.Sword`) (`self.Mesh`) "Holster_Sword" "KeepRelative" "KeepRelative" "KeepRelative" true))

(event `InputAction|Attacking`
  (params (Key :type "Key Structure"))
  (:`Pressed`
    (if (`self.Drawn`)
      (if (not (`self.Attaking`))
        (set `self.Attaking` true)
        (`self.PlayAnimMontage` "/Game/Character/Montages/Standing_Melee_Attack_1_Montage.Standing_Melee_Attack_1_Montage")))))

(event `EndAttack`
  (set `self.Attaking` false))

(fn `UserConstructionScript`)